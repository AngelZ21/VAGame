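; BP_StupidAI is a simple AI character that wanders to random reachable points and can be killed by damage.
; Roam starts on BeginPlay and restarts itself only when a move succeeds.
; AnyDamage sets Health to damage minus Health, an inverted subtraction, then prints a hit or calls Death at zero or below.
; Death disables movement and capsule collision, ragdolls the mesh with an impulse from location plus yaw, and changes its text label.
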(event Custom|Roam
  (AI|AIMoveTo self (.RandomLocation (AI|Navigation|GetRandomReachablePointinRadius (Transformation|GetActorLocation) 2e+05 0 0)) 0 15.0 false
    (:OnSuccess
      (CallFunction|Roam))))

(event Custom|Death
  (bind _mesh (Variables|Character|GetMesh))
  (Pawn|Components|CharacterMovement|DisableMovement (Variables|Character|GetCharacterMovement))
  (Physics|SetSimulatePhysics _mesh true)
  (Physics|AddImpulse _mesh (* (+ (Transformation|GetActorLocation) (.Yaw (Math|Rotator|BreakRotator (Transformation|GetActorRotation)))) 5.0) "None" true)
  (Collision|SetCollisionEnabled (Variables|Collision|GetCapsuleComponent) "NoCollision")
  (Rendering|Components|TextRender|SetText (Variables|Default|GetTextRender) (Variables|Default|GetDead))
  (Collision|SetCollisionEnabled (Variables|Collision|GetCapsuleComponent) "NoCollision"))

(event EventBeginPlay
  (CallFunction|Roam))

(event Collision|EventActorBeginOverlap
  (params (OtherActor :type Actor%20Object%20Reference)))

(event EventTick
  (params (DeltaSeconds :type Float%20%28single-precision%29)))

(event Game|Damage|EventAnyDamage
  (params (Damage :type Float%20%28single-precision%29) (DamageType :type Damage%20Type%20Object%20Reference) (InstigatedBy :type Controller%20Object%20Reference) (DamageCauser :type Actor%20Object%20Reference))
  (Variables|Default|SetHealth (- Damage (Variables|Default|GetHealth)))
  (if (<= (- Damage (Variables|Default|GetHealth)) 0.0)
    (CallFunction|Death)
    (else
      (Development|PrintString "Hit!"))))

(fn ConstructionScript)