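; BP_ShootyAI is an AI character that roams the level and deals contact damage to whatever its capsule hits.
; BeginPlay sets walk speed and starts Roam, which moves to random reachable points and re-triggers itself only on success.
; PawnSensing sightings clear SawAPlayer before calling FollowPlayer, which requires that flag to be true, so the chase move toward the player never runs from that path.
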(event OnSeePawn(PawnSensing)
  (params (Pawn :type Pawn%20Object%20Reference))
  (Variables|Default|SetSaw%20a%20Player? false)
  (CallFunction|FollowPlayer))

(event OnComponentHit(CapsuleComponent)
  (params (HitComponent :type Primitive%20Component%20Object%20Reference) (OtherActor :type Actor%20Object%20Reference) (OtherComp :type Primitive%20Component%20Object%20Reference) (NormalImpulse :type Vector :default "0, 0, 0") (Hit :type Hit%20Result%20Structure%20%28by%20ref%29))
  (Game|Damage|ApplyDamage OtherActor 1e+01 0 0))

(event Custom|Roam
  (AI|AIMoveTo self (.RandomLocation (AI|Navigation|GetRandomReachablePointinRadius (Transformation|GetActorLocation) 2e+05 0 0)) 0 15.0 false
    (:OnSuccess
      (CallFunction|Roam))))

(event Custom|FollowPlayer
  (if (Variables|Default|GetSaw%20a%20Player?)
    (AI|AIMoveTo self "0, 0, 0" (Game|GetPlayerCharacter 0) 5e+04 false)))

(event EventBeginPlay
  (Variables|/Script/Engine.CharacterMovementComponent|SetMaxWalkSpeed (Variables|Character|GetCharacterMovement) 6e+02)
  (CallFunction|Roam))

(event Collision|EventActorBeginOverlap
  (params (OtherActor :type Actor%20Object%20Reference)))

(fn ConstructionScript)