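; Player character Blueprint, despite its PlayerController name, with movement, cooldown dash, ADS, wall-running, temporary hitscan fire and death.
; Tick line-traces sideways while falling to align along walls, lock velocity and remove gravity; Jump launches off them.
; ADS timelines drive spring-arm length alongside walk-speed changes.
; Any damage on authority triggers death unconditionally, with ragdoll, fade, death camera and UI_Dead; wall-run FX functions are empty stubs.
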(event Custom|ChangeHUD
  ;[1 1 1] Change HUD
  (CameraFades|StartCameraFade :self (Game|GetPlayerCameraManager 0) :FromAlpha 1.0 :Duration 0.2 :bHoldWhenFinished true)
  (Components|Activation|SetActive (Variables|Default|GetCamera1) true false)
  (Components|Activation|SetActive (Variables|Default|GetCamera) false false)
  (Utilities|FlowControl|Sequence
    (:then_0
      (Viewport|RemoveAllWidgets)
      (bind _returnvalue (UserInterface|CreateWidget "/Game/UI/UI_Dead.UI_Dead_C"))
      (UserInterface|Viewport|AddtoViewport _returnvalue 0))
    (:then_1
      ;[1 1 1] Death Cam
      (bind _newtrack_0 (Timeline|CamLook Play)
        (:Update
          (Variables|/Script/Engine.SpringArmComponent|SetTargetArmLength (Variables|Default|GetDeathCam) _newtrack_0))))))

(event Custom|Death
  ;[1 1 1] Death
  (Pawn|Components|CharacterMovement|DisableMovement (Variables|Character|GetCharacterMovement))
  (Physics|SetSimulatePhysics (Variables|Character|GetMesh) true)
  (Collision|SetCollisionResponsetoChannel (Variables|Collision|GetCapsuleComponent) "ECC_Pawn" "ECR_Ignore")
  (Utilities|FlowControl|Delay 3.0)
  (Viewport|RemoveAllWidgets))

(event Game|Damage|EventAnyDamage
  (params (Damage :type Float%20%28single-precision%29) (DamageType :type Damage%20Type%20Object%20Reference) (InstigatedBy :type Controller%20Object%20Reference) (DamageCauser :type Actor%20Object%20Reference))
  ;[1 1 1] Damage
  (Networking|SwitchHasAuthority
    (:Authority
      (Development|PrintString "Dead")
      (Variables|Default|SetHealth (Math|Float|Clamp(Float) (- Damage (Variables|Default|GetHealth)) 0.0 (Variables|Default|GetHealth)))
      (if true
        (CameraFades|StartCameraFade :self (Game|GetPlayerCameraManager 0) :ToAlpha 1.0 :Duration 0.1 :bHoldWhenFinished true)
        (Utilities|FlowControl|Delay 0.05)
        (CallFunction|Death)
        (CallFunction|ChangeHUD)))))

(event EventBeginPlay
  ;[0.3412 0.619 1] UI Activiation
  (Rendering|Components|TextRender|SetText (Variables|Default|GetTextRender) (Utilities|Text|ToText(String) (Utilities|Platform|GetPlatformUserName)))
  (Components|Activation|SetActive (Variables|Default|GetCamera) true false)
  (bind _returnvalue (UserInterface|CreateWidget "/Game/UI/UI_HUD.UI_HUD_C"))
  (Utilities|FlowControl|DoOnce false
    (:Completed
      (UserInterface|Viewport|AddtoViewport _returnvalue 0))))

(event EventPossessed
  (params (NewController :type Controller%20Object%20Reference))
  ;[0.3412 0.619 1] UI Activiation
  (Components|Activation|SetActive (Variables|Default|GetCamera) true false)
  (bind _returnvalue (UserInterface|CreateWidget "/Game/UI/UI_HUD.UI_HUD_C"))
  (Utilities|FlowControl|DoOnce false
    (:Completed
      (UserInterface|Viewport|AddtoViewport _returnvalue 0))))

(event Input|ActionEvents|InputActionFire
  (params (Key :type Key%20Structure :default "None"))
  ;[1 0.688 0] Tempoary Firing
  (:Pressed
    (Variables|Default|SetBIsfiring true)
    (if (Variables|Default|GetBIsfiring) :!label _label
      (CallFunction|TempFire)
      (Utilities|FlowControl|Delay 0.1)
      (goto _label)))
  (:Released
    (Variables|Default|SetBIsfiring false)))

(event Input|ActionEvents|InputActionDash
  (params (Key :type Key%20Structure :default "None"))
  ;[1 1 1] Dash
  (:Pressed
    (if (not (Variables|Default|GetIsJumping?))
      (Utilities|FlowControl|DoOnce false :!label _label
        (:Completed
          (CallFunction|Dash)
          (Utilities|FlowControl|Delay 1.0)
          (goto _label Reset))))))

(event Input|ActionEvents|InputActionADS
  (params (Key :type Key%20Structure :default "None"))
  ;[1 1 1] ADS
  (:Pressed
    (Variables|/Script/Engine.CharacterMovementComponent|SetMaxWalkSpeed (Variables|Character|GetCharacterMovement) 3e+02)
    (bind _newtrack_0 (Timeline|ADS%20Cam PlayFromStart)
      (:Update
        (Variables|/Script/Engine.SpringArmComponent|SetTargetArmLength (Variables|Default|GetSpringArm) _newtrack_0))))
  (:Released
    (Variables|/Script/Engine.CharacterMovementComponent|SetMaxWalkSpeed (Variables|Character|GetCharacterMovement) 875.0)
    (bind _newtrack_0_2 (Timeline|Reverse%20ADS PlayFromStart)
      (:Update
        (Variables|/Script/Engine.SpringArmComponent|SetTargetArmLength (Variables|Default|GetSpringArm) _newtrack_0_2)))))

(event Input|AxisEvents|InputAxisForward/Backwards
  (params (AxisValue :type Float%20%28single-precision%29))
  ;[1 0 0] Base Movement
  (Pawn|Input|AddMovementInput (Transformation|GetActorForwardVector) AxisValue false))

(event Input|AxisEvents|InputAxisStrafe
  (params (AxisValue :type Float%20%28single-precision%29))
  ;[1 0 0] Base Movement
  (Pawn|Input|AddMovementInput (Transformation|GetActorRightVector) AxisValue false))

(event Input|AxisEvents|InputAxisCameraTurn
  (params (AxisValue :type Float%20%28single-precision%29))
  ;[1 0 0] Base Movement
  (Pawn|Input|AddControllerYawInput AxisValue))

(event Input|AxisEvents|InputAxisCameraLookup
  (params (AxisValue :type Float%20%28single-precision%29))
  ;[1 0 0] Base Movement
  (Pawn|Input|AddControllerPitchInput AxisValue))

(event Input|KeyboardEvents|K
  (params (Key :type Key%20Structure :default "None"))
  (:Pressed
    ;[1 1 1] Damage
    (Networking|SwitchHasAuthority
      (:Authority
        (Development|PrintString "Dead")
        (Variables|Default|SetHealth (Math|Float|Clamp(Float) (- (stale Game|Damage|EventAnyDamage Damage) (Variables|Default|GetHealth)) 0.0 (Variables|Default|GetHealth)))
        (if true
          (CameraFades|StartCameraFade :self (Game|GetPlayerCameraManager 0) :ToAlpha 1.0 :Duration 0.1 :bHoldWhenFinished true)
          (Utilities|FlowControl|Delay 0.05)
          (CallFunction|Death)
          (CallFunction|ChangeHUD))))))

(event Input|KeyboardEvents|Backspace
  (params (Key :type Key%20Structure :default "None"))
  ;[0.3412 0.619 1] UI Activiation
  (:Pressed
    (bind _returnvalue (UserInterface|CreateWidget "/Game/UI/UI_Pause.UI_Pause_C"))
    (UserInterface|Viewport|AddtoViewport _returnvalue 0)
    (Input|DisableInput 0)))

(event Custom|Offwall
  (bind _charactermovement (Variables|Character|GetCharacterMovement))
  ;[1 1 1] Wallrun [-Thanks to BlueprintUE-]
  ;;[0 0.8216 1] WallRunning OffWall Condition
  (Variables|/Script/Engine.CharacterMovementComponent|SetGravityScale _charactermovement 1.0)
  (Class|MovementComponent|SetPlaneConstraintNormal _charactermovement "0, 0, 0")
  (CallFunction|StopWallRunFX))

(event EventTick
  (params (DeltaSeconds :type Float%20%28single-precision%29))
  (bind _returnvalue (Transformation|GetActorForwardVector))
  (bind _returnvalue_2 (Transformation|GetActorLocation))
  (bind _returnvalue_3 (Transformation|GetActorLocation))
  (bind _returnvalue_4 (Transformation|GetActorForwardVector))
  (bind _charactermovement (Variables|Character|GetCharacterMovement))
  (bind _charactermovement_2 (Variables|Character|GetCharacterMovement))
  (bind _returnvalue_5 (* _returnvalue 1e+03))
  (bind _returnvalue_6 (* _returnvalue_4 1e+03))
  ;[1 1 1] Wallrun [-Thanks to BlueprintUE-]
  ;;[0.18 0.6 0.9] Event Tick
  (|CallParentFunction DeltaSeconds)
  (CallFunction|UpdateColoringSystem)
  (CallFunction|UpdateHeldObjectAnimations)
  (if (AI|Components|NavMovement|IsFalling (Variables|Character|GetCharacterMovement))
    (Utilities|FlowControl|Sequence
      (:then_0
        (if (not (Variables|Default|GetLeftSide?))
          ;;[1 1 1] Right Side Wall Detection
          (bind (_outhit _returnvalue_7) (Collision|LineTraceByChannel _returnvalue_3 (+ _returnvalue_3 (* (Transformation|GetActorRightVector) 5e+01)) "TraceTypeQuery1" false 0 "None" true "(R=0.000000,G=1.000000,B=0.278894,A=1.000000)"))
          ;;[1 0.6424 0] WallRun RightSide
          (if _returnvalue_7
            (Variables|Default|SetRightSide? true)
            (Variables|Default|SetOnRightSide true)
            (if (not (Variables|Default|GetIsJumpingOffWall))
              (CallFunction|TriggerWallRunFX)
              (Transformation|SetActorRotation (Math|Rotator|MakeRotator 0.0 0.0 (+ (.yaw (Math|Conversions|RotationFromXVector (.Normal (Collision|BreakHitResult _outhit)))) 9e+01)))
              (Variables|/Script/Engine.MovementComponent|SetVelocity _charactermovement_2 (Math|Vector|MakeVector (.x _returnvalue_5) (.y _returnvalue_5) 0.0))
              (Variables|/Script/Engine.CharacterMovementComponent|SetGravityScale _charactermovement_2 0.0)
              (Class|MovementComponent|SetPlaneConstraintNormal _charactermovement_2 "0, 0,1.000000"))
            (else
              (Variables|Default|SetRightSide? false)
              (CallFunction|Offwall)))))
      (:then_1
        (if (not (Variables|Default|GetRightSide?))
          ;;[1 1 1] Left Side Wall Detection
          (bind (_outhit_2 _returnvalue_8) (Collision|LineTraceByChannel _returnvalue_2 (+ _returnvalue_2 (* (Transformation|GetActorRightVector) -5e+01)) "TraceTypeQuery1" false 0 "None" true "(R=1.000000,G=0.266356,B=0.000000,A=1.000000)"))
          ;;[0 1 0.09324] WallRun LeftSide
          (if _returnvalue_8
            (Variables|Default|SetLeftSide? true)
            (Variables|Default|SetOnRightSide false)
            (if (not (Variables|Default|GetIsJumpingOffWall))
              (CallFunction|TriggerWallRunFX)
              (Transformation|SetActorRotation (Math|Rotator|MakeRotator 0.0 0.0 (+ (.yaw (Math|Conversions|RotationFromXVector (.Normal (Collision|BreakHitResult _outhit_2)))) -9e+01)))
              (Variables|/Script/Engine.MovementComponent|SetVelocity _charactermovement (Math|Vector|MakeVector (.x _returnvalue_6) (.y _returnvalue_6) 0.0))
              (Variables|/Script/Engine.CharacterMovementComponent|SetGravityScale _charactermovement 0.0)
              (Class|MovementComponent|SetPlaneConstraintNormal _charactermovement "0, 0,1.000000"))
            (else
              (Variables|Default|SetLeftSide? false)
              (CallFunction|Offwall))))))))

(event Input|ActionEvents|InputActionJump
  (params (Key :type Key%20Structure :default "None"))
  (bind _returnvalue (Transformation|GetActorRightVector))
  (bind _returnvalue_2 (Transformation|GetActorRightVector))
  (bind _onrightside (Variables|Default|GetOnRightSide))
  (bind _returnvalue_3 (* _returnvalue_2 -3.5e+02))
  (bind _returnvalue_4 (* _returnvalue 3.5e+02))
  (bind _returnvalue_5 (select _onrightside _returnvalue_3 _returnvalue_4))
  ;[1 1 1] Wallrun [-Thanks to BlueprintUE-]
  ;;[1 0.9776 0] Set Jump While WallRunning
  (:Pressed
    (if (or (Variables|Default|GetRightSide?) (Variables|Default|GetLeftSide?))
      (Variables|Default|SetIsJumpingOffWall true)
      (Character|LaunchCharacter (Math|Vector|MakeVector (.x _returnvalue_5) (.y _returnvalue_5) 7e+02) false true)
      (Variables|/Script/Engine.MovementComponent|SetVelocity (Variables|Character|GetCharacterMovement) (/ (Variables|/Script/Engine.MovementComponent|GetVelocity (Variables|Character|GetCharacterMovement)) 1.0))
      (Variables|Default|SetIsJumpingOffWall false)
      (else
        ;;[1 1 1] Jump Action
        (Character|Jump)))))

(fn ConstructionScript)

(fn Dash
  (Character|LaunchCharacter (* (+ (* (Transformation|GetActorForwardVector) (Input|AxisValues|GetForward/Backwards)) (* (Transformation|GetActorRightVector) (Input|AxisValues|GetStrafe))) 2e+03) false true))

(fn TempFire
  (bind _camera (Variables|Default|GetCamera))
  (bind (_outhit _returnvalue) (Collision|LineTraceByChannel (Transformation|GetWorldLocation _camera) (* (Math|Vector|GetForwardVector _camera) 5e+03) "TraceTypeQuery2" true 0 "ForDuration"))
  (if _returnvalue
    (Game|Damage|ApplyDamage (.HitActor (Collision|BreakHitResult _outhit)) 5.0 0 0)))

(fn UpdateColoringSystem)

(fn UpdateHeldObjectAnimations)

(fn TriggerWallRunFX)

(fn StopWallRunFX)