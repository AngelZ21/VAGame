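; BPC_Limb is a limb health component that tracks a TotalHP pool and signals death when it is depleted.
; The AnyPointDM event passes incoming damage to UpdateTotalHP, then prints the resulting HP; its BulletHit input is unused.
; UpdateTotalHP subtracts damage by clamping TotalHP between zero and TotalHP minus Damage, and calls the CallOnDeath dispatcher whenever the result is zero or below.
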(event Custom|Event%20Any%20Point%20DM
  (params (Damage :type Float%20%28single-precision%29) (BulletHit :type Hit%20Result%20Structure))
  (CallFunction|UpdateTotalHP Damage)
  (Development|PrintString (Utilities|String|ToString(Float) (Variables|Default|GetTotalHP))))

(event EventBeginPlay)

(event EventTick
  (params (DeltaSeconds :type Float%20%28single-precision%29)))

(fn UpdateTotalHP
  (params (Damage :type Float%20%28single-precision%29))
  (bind _output_get (Variables|Default|SetTotalHP (Math|Float|Clamp(Float) (Variables|Default|GetTotalHP) 0.0 (- (Variables|Default|GetTotalHP) Damage))))
  (if (<= _output_get 0.0)
    (Default|CallCall"OnDeath")))